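; CubeBP is an actor that travels along a spline path and destroys itself when its cube is hit by a BallBP.
; On BeginPlay it finds a SplinePathBP and starts a timeline, with play rate scaled by TimeToCompleteInSeconds.
; Each update maps the timeline track to spline distance, setting location in world space and rotation in local space.
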(event OnComponentHit(Cube)
  (params (HitComponent :type Primitive%20Component%20Object%20Reference) (OtherActor :type Actor%20Object%20Reference) (OtherComp :type Primitive%20Component%20Object%20Reference) (NormalImpulse :type Vector :default "0, 0, 0") (Hit :type Hit%20Result%20Structure%20%28by%20ref%29))
  (Utilities|Casting|CastToBallBP OtherActor)
  (Actor|DestroyActor))

(event Custom|MoveObject
  (bind _splineref (Variables|Default|GetSplineREF))
  (bind _spline (Variables|/Game/Blueprints/SplinePathBP.SplinePathBP_C|GetSpline _splineref))
  (Components|Timeline|SetPlayRate (Variables|Default|GetMove%20Object%201) (/ 1.0 (Variables|Default|GetTime%20To%20Complete%20%28In%20Seconds%29)))
  (bind _move_track (Timeline|Move%20Object%201 Play)
    (:Update
      (Transformation|SetActorTransform (Math|Transform|MakeTransform (Spline|GetLocationatDistanceAlongSpline _spline (Math|Float|Lerp 0.0 (Spline|GetSplineLength (Variables|/Game/Blueprints/SplinePathBP.SplinePathBP_C|GetSpline (Variables|Default|GetSplineREF))) _move_track) "World") (Spline|GetRotationatDistanceAlongSpline _spline (Math|Float|Lerp 0.0 (Spline|GetSplineLength (Variables|/Game/Blueprints/SplinePathBP.SplinePathBP_C|GetSpline (Variables|Default|GetSplineREF))) _move_track) "Local") "1,1,1")))))

(event EventBeginPlay
  (bind _returnvalue (Actor|GetActorOfClass "/Game/Blueprints/SplinePathBP.SplinePathBP_C"))
  (Variables|Default|SetSplineREF _returnvalue)
  (CallFunction|MoveObject))

(fn ConstructionScript)